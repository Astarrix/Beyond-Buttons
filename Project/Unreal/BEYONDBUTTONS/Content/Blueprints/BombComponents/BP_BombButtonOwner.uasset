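; BP_BombButtonOwner is a bomb component with nine buttons that each toggle between on and off when interacted with.
; The construction script fills an empty ButtonStates map from the button meshes and gives each a dynamic material coloured by its state.
; Interaction flips the hit button's state, recolours it green or dark grey, and fires the EDButtonPushed dispatcher with the button's key index and new state.
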(event `/Game/Tools/_BPI.Interaction`
  (params (Interactor :type "Object Object Reference") (HitComponent :type "PrimitiveComponent Object Reference"))
  (bind _asstatic_mesh_component (cast `StaticMeshComponent` HitComponent))
  (bind _keys (`BlueprintMapLibrary.Map_Keys` (`self.ButtonStates`)))
  (if (`KismetArrayLibrary.Array_Contains` _keys _asstatic_mesh_component)
    (`self.ToggleButtonState` _asstatic_mesh_component)))

(event `ToggleButtonState`
  (params (Button :type "StaticMeshComponent Object Reference"))
  (bind _buttonstates (`self.ButtonStates`))
  (bind (_value _returnvalue) (`BlueprintMapLibrary.Map_Find` _buttonstates Button))
  (if _returnvalue
    (`BlueprintMapLibrary.Map_Add` _buttonstates Button (not _value))
    (`self.ToggleButtonColour` Button)
    (bind _keys (`BlueprintMapLibrary.Map_Keys` _buttonstates))
    (`self.ED_ButtonPushed` (`KismetArrayLibrary.Array_Find` _keys Button) (`BlueprintMapLibrary.Map_Find` _buttonstates Button))))

(event `ToggleButtonColour`
  (params (Button :type "StaticMeshComponent Object Reference"))
  (bind (_value _returnvalue) (`BlueprintMapLibrary.Map_Find` (`self.ButtonStates`) Button))
  (if _returnvalue
    (`MeshComponent.SetVectorParameterValueOnMaterials` Button "Colour" (`KismetMathLibrary.Conv_LinearColorToVector` (`KismetMathLibrary.SelectColor` (struct :`R` 0.191954 :`G` 1.0 :`B` 0.124008 :`A` 1.0) (struct :`R` 0.072917 :`G` 0.072917 :`B` 0.072917 :`A` 1.0) _value)))))

(fn `UserConstructionScript`
  (if (`BlueprintMapLibrary.Map_IsEmpty` (`self.ButtonStates`))
    (bind _output_get (set `self.ButtonStates` (`|MakeMap` (`self.BTN_1`) false (`self.BTN_2`) false (`self.BTN_3`) false (`self.BTN_4`) false (`self.BTN_5`) false (`self.BTN_6`) false (`self.BTN_7`) false (`self.BTN_8`) false (`self.BTN_9`))))
    (bind _keys (`BlueprintMapLibrary.Map_Keys` _output_get))
    (for _array_element _keys
      (bind _returnvalue (`KismetMaterialLibrary.CreateDynamicMaterialInstance` "/Game/Assets/KayKitMiniGameVarietyPack/M_Dynamic.M_Dynamic"))
      (`PrimitiveComponent.SetMaterial` _array_element 0 _returnvalue)
      (`MaterialInstanceDynamic.SetVectorParameterValue` (cast `MaterialInstanceDynamic` (`PrimitiveComponent.GetMaterial` _array_element 0) :!pure true) "Colour" (`KismetMathLibrary.SelectColor` (struct :`R` 0.191954 :`G` 1.0 :`B` 0.124008 :`A` 1.0) (struct :`R` 0.072917 :`G` 0.072917 :`B` 0.072917 :`A` 1.0) (`BlueprintMapLibrary.Map_Find` (`self.ButtonStates`) _array_element))))))