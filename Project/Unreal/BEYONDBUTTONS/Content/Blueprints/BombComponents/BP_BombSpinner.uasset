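; BP_BombSpinner is a bomb component whose static mesh turns a quarter turn around its yaw axis on each interaction.
; Interaction plays the Spin timeline only while the component is active and no spin is already running, lerping yaw from the stored position.
; The stored position starts at the mesh's initial yaw and advances when each spin finishes, with angles wrapped to a full circle.
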(event `self.ReceiveBeginPlay`
  (set `self.CurrentPosition` (.yaw (`SceneComponent.RelativeRotation` (`self.StaticMesh`)))))

(event `/Game/Tools/_BPI.Interaction`
  (params (Interactor :type "Object Object Reference") (HitComponent :type "PrimitiveComponent Object Reference"))
  (bind _currentposition (`self.CurrentPosition`))
  (if (`self.isActive`)
    (if (not (`TimelineComponent.IsPlaying` (`self.Spin`)))
      (bind (_direction _movement) (`Timeline|Spin` :!via `PlayFromStart`)
        (:`Update`
          (`SceneComponent.K2_SetRelativeRotation` (`self.StaticMesh`) (`KismetMathLibrary.MakeRotator` 0.0 0.0 (`KismetMathLibrary.FWrap` (`KismetMathLibrary.Lerp` _currentposition (+ _currentposition 90.0) _movement) 0.0 360.0)) false false))
        (:`Finished`
          (set `self.CurrentPosition` (`KismetMathLibrary.FWrap` (+ (`self.CurrentPosition`) 90.0) 0.0 360.0)))))))

(fn `UserConstructionScript`)