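; BP_BombWireOwner is a bomb component that owns eight cuttable wires and tracks whether each has been cut.
; The construction script fills an empty WireStates map, keyed by the wire static mesh components.
; An interaction on a tracked wire cuts it only once, setting its state and swapping its mesh to mark it.
; Each cut fires the EDWireCut dispatcher with the wire's index in the map keys.
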(event `/Game/Tools/_BPI.Interaction`
  (params (Interactor :type "Object Object Reference") (HitComponent :type "PrimitiveComponent Object Reference"))
  (bind _asstatic_mesh_component (cast `StaticMeshComponent` HitComponent))
  (bind _keys (`BlueprintMapLibrary.Map_Keys` (`self.WireStates`)))
  (if (`KismetArrayLibrary.Array_Contains` _keys _asstatic_mesh_component)
    (`self.AttemptCutWire` _asstatic_mesh_component)))

(event `AttemptCutWire`
  (params (SelectedWire :type "StaticMeshComponent Object Reference"))
  (bind (_value _returnvalue) (`BlueprintMapLibrary.Map_Find` (`self.WireStates`) SelectedWire))
  (if (and (not _value) _returnvalue)
    (`self.CutWire` SelectedWire)))

(event `CutWire`
  (params (SelectedWire :type "StaticMeshComponent Object Reference"))
  (bind _wirestates (`self.WireStates`))
  (`BlueprintMapLibrary.Map_Add` _wirestates SelectedWire true)
  (`StaticMeshComponent.SetStaticMesh` SelectedWire "/Game/Assets/KayKitMiniGameVarietyPack/arrow_teamBlue.arrow_teamBlue")
  (bind _keys (`BlueprintMapLibrary.Map_Keys` _wirestates))
  (`self.ED_WireCut` (`KismetArrayLibrary.Array_Find` _keys SelectedWire)))

(fn `UserConstructionScript`
  (if (`BlueprintMapLibrary.Map_IsEmpty` (`self.WireStates`))
    (set `self.WireStates` (`|MakeMap` (`self.Wire_1`) false (`self.Wire_2`) false (`self.Wire_3`) false (`self.Wire_4`) false (`self.Wire_5`) false (`self.Wire_6`) false (`self.Wire_7`) false (`self.Wire_8`)))))