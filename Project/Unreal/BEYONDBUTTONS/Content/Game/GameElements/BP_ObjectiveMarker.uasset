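; BP_ObjectiveMarker is an objective marker that displays an arrow widget and completes an objective when its Box trigger is overlapped.
; On BeginPlay it caches GM_MAIN, then creates a green-tinted WUI_Arrow and assigns it to its Widget component.
; Any overlap, with no actor filtering, passes the current objective key plus the next key and text to the game mode's CompleteObjective, then hides the arrow.
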(event `CreateWidget`
  (bind _returnvalue (`|CreateWidget` "/Game/UI/WUI_Arrow.WUI_Arrow_C"))
  (bind _output_get (set `self.WUI_Arrow` _returnvalue))
  (`/Game/UI/WUI_Arrow.SetMarkerColour` _output_get (struct :`G` 1.0 :`B` 0.57512 :`A` 1.0))
  (`WidgetComponent.SetWidget` (`self.Widget`) _returnvalue))

(event `self.ReceiveBeginPlay`
  (`self.CreateRefs`)
  (`self.CreateWidget`))

(event `CreateRefs`
  (bind _asgm_main (cast `/Game/Game/Core/GM_MAIN` (`GameplayStatics.GetGameMode`)))
  (set `self.As GM MAIN` _asgm_main))

(event `self.Box.OnComponentBeginOverlap`
  (params (OverlappedComponent :type "PrimitiveComponent Object Reference") (OtherActor :type "Actor Object Reference") (OtherComp :type "PrimitiveComponent Object Reference") (OtherBodyIndex :type Integer) (bFromSweep :type Boolean) (SweepResult :type "HitResult Structure (by ref)"))
  (`/Game/Game/Core/GM_MAIN.CompleteObjective` (`self.As GM MAIN`) (`self.CurrentObjectiveKey`) false (`self.New Objective Key`) (`self.New Objective Text`))
  (`/Game/UI/WUI_Arrow.SetMarkerVisibility` (`self.WUI_Arrow`) false))

(fn `UserConstructionScript`)