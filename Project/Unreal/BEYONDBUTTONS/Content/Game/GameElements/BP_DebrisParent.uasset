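; BP_DebrisParent is a base debris actor that can scatter itself to a spot free of other debris.
; Disperse shifts the actor by a random offset on each axis, then sphere-tests its StaticMesh bounds against other physics-body debris.
; While an overlap is found it repeats from the new location with no retry limit, drawing each test as a red (blocked) or green (clear) debug sphere.
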(event `Disperse`
  (bind (_origin _boxextent _sphereradius) (`KismetSystemLibrary.GetComponentBounds` (`self.StaticMesh`)))
  (`self.K2_SetActorLocation` (`KismetMathLibrary.MakeVector` (+ (.x (`self.K2_GetActorLocation`)) (`KismetMathLibrary.RandomFloatInRange` -200.0 200.0)) (+ (.y (`self.K2_GetActorLocation`)) (`KismetMathLibrary.RandomFloatInRange` -200.0 200.0)) (+ (.z (`self.K2_GetActorLocation`)) (`KismetMathLibrary.RandomFloatInRange` -200.0 200.0))) :!label _label)
  (bind (_outactors _returnvalue) (`KismetSystemLibrary.SphereOverlapActors` _origin _sphereradius (`|MakeArray` "ObjectTypeQuery4" :!type "EObjectTypeQuery Enum") "BP_DebrisParent_C" (`|MakeArray` self :!type "Actor Object Reference")))
  (`KismetSystemLibrary.DrawDebugSphere` _origin _sphereradius 12 (`KismetMathLibrary.SelectColor` (struct :`R` 1.0 :`A` 1.0) (struct :`G` 1.0 :`A` 1.0) _returnvalue) 2.0 2.0)
  (if _returnvalue
    (goto _label)))

(fn `UserConstructionScript`)