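; BP_Pickup is a base pickup that triggers when BP_Astronaut overlaps its box, calling the empty InteractedWith hook and displaying text through BPCText.
; Non-persistent pickups then destroy themselves.
; SetPickupInfo supplies the text, persistence and custom-depth stencil highlight, while BeginPlay randomises rotation and caches GM_MAIN.
; The construction script centres the mesh, fits the padded box to its bounds and flattens the actor to Z zero.
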(event `self.ReceiveBeginPlay`
  (`self.K2_SetActorRotation` (`KismetMathLibrary.MakeRotator` (`KismetMathLibrary.RandomFloatInRange` 0.0 360.0) (`KismetMathLibrary.RandomFloatInRange` 0.0 360.0) (`KismetMathLibrary.RandomFloatInRange` 0.0 360.0)))
  (set `self.As GM MAIN` (cast `/Game/Game/Core/GM_MAIN` (`GameplayStatics.GetGameMode`) :!pure true)))

(event `SetPickupInfo`
  (params (inText :type String) (HighlightingColour :type Byte) (isPersistent :type Boolean))
  (set `self.isPersistent` isPersistent)
  (set `/Game/Game/GameElements/BPC_Text.DisplayText` inText (`self.BPC_Text`))
  (`PrimitiveComponent.SetCustomDepthStencilValue` (`self.StaticMesh`) (`KismetMathLibrary.Conv_ByteToInt` HighlightingColour)))

(event `self.Box.OnComponentBeginOverlap`
  (params (OverlappedComponent :type "PrimitiveComponent Object Reference") (OtherActor :type "Actor Object Reference") (OtherComp :type "PrimitiveComponent Object Reference") (OtherBodyIndex :type Integer) (bFromSweep :type Boolean) (SweepResult :type "HitResult Structure (by ref)"))
  (bind _ispersistent (`self.isPersistent`))
  (cast `/Game/Game/Player/BP_Astronaut` OtherActor)
  (`self.InteractedWith`)
  (`/Game/Game/GameElements/BPC_Text.Display` (`self.BPC_Text`) (not _ispersistent))
  (if (not _ispersistent)
    (`self.K2_DestroyActor`)))

(fn `InteractedWith`)

(fn `UserConstructionScript`
  (bind _staticmesh (`self.StaticMesh`))
  (`SceneComponent.K2_SetRelativeLocation` (`self.StaticMesh`) (* (`KismetMathLibrary.BreakBoxSphereBounds` (`StaticMesh.GetBounds` (`StaticMeshComponent.StaticMesh` (`self.StaticMesh`)))) (-1.0 -1.0 -1.0)) false false)
  (`SceneComponent.K2_SetRelativeLocation` (`self.Box`) (0.0 0.0 0.0) false false)
  (`BoxComponent.SetBoxExtent` (`self.Box`) (+ (`.BoxExtent` (`KismetMathLibrary.BreakBoxSphereBounds` (`StaticMesh.GetBounds` (`StaticMeshComponent.StaticMesh` _staticmesh)))) 50.0) true)
  (`SceneComponent.K2_SetRelativeRotation` (`self.Box`) (`SceneComponent.RelativeRotation` _staticmesh) false false)
  (`self.K2_SetActorLocation` (* (`self.K2_GetActorLocation`) (1.0 1.0 0.0))))