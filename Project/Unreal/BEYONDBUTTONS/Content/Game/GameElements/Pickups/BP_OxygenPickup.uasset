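; Oxygen pickup that restores a fixed amount of the player's remaining oxygen when interacted with.
; On BeginPlay it passes a random flavour message, a highlight colour and a non-persistent flag to the inherited SetPickupInfo.
; InteractedWith adds the oxygen to the player reached through the game mode reference, clamps it to the valid range, then runs the parent interaction logic.
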(event `self.ReceiveBeginPlay`
  (`parent.ReceiveBeginPlay`)
  (`self.SetPickupInfo` (`KismetArrayLibrary.Array_Random` (`|MakeArray` "Good to have some oxygen!" "Oxygen tanks restored!" "Ah feels better, I can breathe again!" "*Deep Breath* much better!" "O2 Levels Increased!")) 4))

(fn `InteractedWith`
  (bind _as_playermain (`/Game/Game/Core/GM_MAIN.As PLAYERMAIN` (`self.As GM MAIN`)))
  (set `/Game/Game/Player/BP_Astronaut.OxygenRemaining` (`KismetMathLibrary.FClamp` (+ (`/Game/Game/Player/BP_Astronaut.OxygenRemaining` _as_playermain) 25.0) 0.0 100.0) _as_playermain)
  (`parent.InteractedWith`))

(fn `UserConstructionScript`
  (`parent.UserConstructionScript`))