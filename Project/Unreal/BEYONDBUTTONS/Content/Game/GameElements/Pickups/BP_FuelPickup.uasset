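; Fuel pickup Blueprint that adds a fixed amount of fuel to the player's thrusters when interacted with.
; On BeginPlay it passes a randomly chosen flavour line and a highlight colour to the parent's pickup info, marked non-persistent.
; Its InteractedWith override reaches the thrusters component through the game mode's player reference, then defers to the parent implementation.
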(event `self.ReceiveBeginPlay`
  (`parent.ReceiveBeginPlay`)
  (`self.SetPickupInfo` (`KismetArrayLibrary.Array_Random` (`|MakeArray` "Fuel levels increased!" "Topped off the tanks! good job!" "That'll keep us going a while longer!" "Always good to be stocked up on fuel!" "Good job we found that fuel!")) 3))

(fn `InteractedWith`
  (`/Game/Game/Player/BPC_Thrusters.FuelPickup` (`/Game/Game/Player/BP_Astronaut.BPC_Thrusters` (`/Game/Game/Core/GM_MAIN.As PLAYERMAIN` (`self.As GM MAIN`))) 25.0)
  (`parent.InteractedWith`))

(fn `UserConstructionScript`
  (`parent.UserConstructionScript`))