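; BP_KeycodePickup is a pickup that reveals the main door's code, labelled as a main door keycard.
; On BeginPlay it waits one tick, then looks up "DoorCode" in the GMMAIN game mode's Codes map.
; It passes that text to SetPickupInfo as a non-persistent pickup, leaving interaction handling to the parent class.
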(event `self.ReceiveBeginPlay`
  (`parent.ReceiveBeginPlay`)
  (`KismetSystemLibrary.DelayUntilNextTick`)
  (`self.SetPickupInfo` (`KismetStringLibrary.Concat_StrStr` "Main Door Keycard: " (`BlueprintMapLibrary.Map_Find` (`/Game/Game/Core/GM_MAIN.Codes` (`self.As GM MAIN`)) "DoorCode"))))

(fn `InteractedWith`
  (`parent.InteractedWith`))

(fn `UserConstructionScript`
  (`parent.UserConstructionScript`))