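; BP_Door is a two-panel door, labelled "Shuttle Door", that opens once when it receives a correct code.
; It reads its code from GM_MAIN one tick after BeginPlay.
; When BP_Astronaut overlaps the box, it registers with the game mode's ArduinoInterface as a listener for that code.
; A successful CodeCheck plays the Slide timeline, which fakes sliding by shrinking both holders' X scale to zero.
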(event `OpenDoor`
  (bind _l_doorholder (`self.L_DoorHolder`))
  (bind _r_doorholder (`self.R_DoorHolder`))
  (bind (_relativescale3d_x _relativescale3d_y _relativescale3d_z) (`KismetMathLibrary.BreakVector` (`SceneComponent.RelativeScale3D` _r_doorholder)))
  (bind (_relativescale3d_x_2 _relativescale3d_y_2 _relativescale3d_z_2) (`KismetMathLibrary.BreakVector` (`SceneComponent.RelativeScale3D` _l_doorholder)))
  (`/Engine/EditorBlueprintResources/StandardMacros.DoOnce` false
    (:`Completed`
      (bind (_direction _float) (`Timeline|Slide` :!via `PlayFromStart`)
        (:`Update`
          (bind _returnvalue (`KismetMathLibrary.Lerp` 1.75 0.0 _float))
          (`SceneComponent.SetRelativeScale3D` _r_doorholder (`KismetMathLibrary.MakeVector` _returnvalue _relativescale3d_y _relativescale3d_z))
          (`SceneComponent.SetRelativeScale3D` _l_doorholder (`KismetMathLibrary.MakeVector` _returnvalue _relativescale3d_y_2 _relativescale3d_z_2)))))))

(event `/Game/Tools/_BPI.CodeCheck`
  (params (isCorrect :type Boolean) (inCode :type String) (CorrectCode :type String))
  (if isCorrect
    (`self.OpenDoor`)))

(event `self.ReceiveBeginPlay`
  (`KismetSystemLibrary.DelayUntilNextTick`)
  (bind _output_get (set `self.As GM MAIN` (cast `/Game/Game/Core/GM_MAIN` (`GameplayStatics.GetGameMode`) :!pure true)))
  (set `self.DoorCode` (`BlueprintMapLibrary.Map_Find` (`/Game/Game/Core/GM_MAIN.Codes` _output_get) "DoorCode")))

(event `self.Box.OnComponentBeginOverlap`
  (params (OverlappedComponent :type "PrimitiveComponent Object Reference") (OtherActor :type "Actor Object Reference") (OtherComp :type "PrimitiveComponent Object Reference") (OtherBodyIndex :type Integer) (bFromSweep :type Boolean) (SweepResult :type "HitResult Structure (by ref)"))
  (cast `/Game/Game/Player/BP_Astronaut` OtherActor)
  (`/Game/Game/Core/BP_ArduinoInterface.RegisterCodeListener` (`/Game/Game/Core/GM_MAIN.ArduinoInterface` (`self.As GM MAIN`)) self (`self.DoorCode`) "Shuttle Door"))

(fn `UserConstructionScript`)