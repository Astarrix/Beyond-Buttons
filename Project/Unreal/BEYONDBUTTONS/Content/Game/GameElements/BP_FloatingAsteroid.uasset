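; BP_FloatingAsteroid is an asteroid actor that slowly tumbles, with its look and spin randomized at construction.
; The construction script picks one of thirteen asteroid meshes and scales it uniformly so its bounding sphere matches Radius.
; A dynamic material instance, created only if missing, receives an InverseScale parameter derived from Radius.
; RotatingMovement gets a random rotation rate on each axis.
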(fn `UserConstructionScript`
  (locals (Mesh :type "StaticMesh Object Reference") (AsteroidMaterial :type "MaterialInstanceDynamic Object Reference"))
  (`|ExecutionSequence`
    (:`then_0`
      (`local.AsteroidMaterial`
        (:`then`
          _)
        (:`else`
          (bind _returnvalue (`KismetMaterialLibrary.CreateDynamicMaterialInstance` "/Game/Assets/Materials/Asteroids_Mat.Asteroids_Mat"))
          (bind _output_get (set `local.AsteroidMaterial` _returnvalue))))
      (`PrimitiveComponent.SetMaterial` (`self.AsteroidMesh`) 0 _output_get))
    (:`then_1`
      (bind _output_get_2 (set `local.Mesh` (`KismetArrayLibrary.Array_Random` (`|MakeArray` "/Game/Assets/Meshes/Asteroids/SM_Asteroid_1.SM_Asteroid_1" "/Game/Assets/Meshes/Asteroids/SM_Asteroid_2.SM_Asteroid_2" "/Game/Assets/Meshes/Asteroids/SM_Asteroid_3.SM_Asteroid_3" "/Game/Assets/Meshes/Asteroids/SM_Asteroid_4.SM_Asteroid_4" "/Game/Assets/Meshes/Asteroids/SM_Asteroid_5.SM_Asteroid_5" "/Game/Assets/Meshes/Asteroids/SM_Asteroid_6.SM_Asteroid_6" "/Game/Assets/Meshes/Asteroids/SM_Asteroid_7.SM_Asteroid_7" "/Game/Assets/Meshes/Asteroids/SM_Asteroid_8.SM_Asteroid_8" "/Game/Assets/Meshes/Asteroids/SM_Asteroid_9.SM_Asteroid_9" "/Game/Assets/Meshes/Asteroids/SM_Asteroid_10.SM_Asteroid_10" "/Game/Assets/Meshes/Asteroids/SM_Asteroid_11.SM_Asteroid_11" "/Game/Assets/Meshes/Asteroids/SM_Asteroid_12.SM_Asteroid_12" "/Game/Assets/Meshes/Asteroids/SM_Asteroid_13.SM_Asteroid_13" :!type "StaticMesh Object Reference"))))
      (`StaticMeshComponent.SetStaticMesh` (`self.AsteroidMesh`) _output_get_2))
    (:`then_2`
      ;[1 1 1] Uniform Size
      (`SceneComponent.SetRelativeScale3D` (`self.AsteroidMesh`) (`KismetMathLibrary.Conv_DoubleToVector` (/ (`self.Radius`) (`.SphereRadius` (`KismetMathLibrary.BreakBoxSphereBounds` (`StaticMesh.GetBounds` (`local.Mesh`))))))))
    (:`then_3`
      (`MaterialInstanceDynamic.SetScalarParameterValue` (`local.AsteroidMaterial`) "InverseScale" (/ 100.0 (`self.Radius`))))
    (:`then_4`
      (set `RotatingMovementComponent.RotationRate` (`KismetMathLibrary.MakeRotator` (`KismetMathLibrary.RandomFloatInRange` -20.0 20.0) (`KismetMathLibrary.RandomFloatInRange` -20.0 20.0) (`KismetMathLibrary.RandomFloatInRange` -20.0 20.0)) (`self.RotatingMovement`)))))