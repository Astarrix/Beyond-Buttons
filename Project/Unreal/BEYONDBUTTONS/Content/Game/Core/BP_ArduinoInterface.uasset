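; BP_ArduinoInterface links the game to an Arduino over SerialCOM, with a debug override that skips connection.
; Init scans COM ports, recursively tests each for a handshake key, replies to the match, and retries on a timer if none is found.
; A fast looping timer reads lines and routes them by prefix; button bitmasks are only debug-printed and commands are stubbed.
; It also sends outgoing commands, plus a terminator before closing on teardown.
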(event `Init`
  ;[1 0.5 0.5] Init
  (if (not (`self.bOverride`))
    (`self.ED_BeginSearch`)
    (bind (_foundports _openableports) (`self.GetOpenablePorts` 16))
    (if _foundports
      (`self.TestPortsForHandshake` 0 _openableports)
      (else
        (`KismetSystemLibrary.PrintText` "FAILED TO FIND ANY AVAILABLE PORTS" (`self.PrintingDebug`) false (struct :`R` 1.0 :`A` 1.0) 5.0 :!label _label)
        (`self.ED_Retrying`)
        (`KismetSystemLibrary.K2_SetTimerDelegate` (`|CreateDelegate` :!event `Init`) 5.0)))
    (else
      (`self.ED_Connected`))))

(event `Failed`
  ;[1 0.5 0.5] Init
  (goto _label))

(event `ContinueExecutionWithBoundPort`
  (params (ConnectedPort :type "SerialCom Object Reference"))
  ;[1 0.5 0.5] Init
  (bind _success (`self.ReturnHandshake` ConnectedPort))
  (if _success
    (set `self.ConnectedPort` ConnectedPort)
    (`self.ED_Connected`)
    (`self.BeginReadSerial`)
    (else
      (`KismetSystemLibrary.PrintText` "FAILED TO RETURN HANDSHAKE" (`self.PrintingDebug`) false (struct :`R` 1.0 :`A` 1.0) 100000.0))))

(event `self.ReceiveDestroyed`
  ;[0.5 1 0.5] Game End Send Close
  (`self.CloseClean` :!label _label_2))

(event `self.ReceiveEndPlay`
  (params (EndPlayReason :type "EEndPlayReason Enum" :default "Destroyed"))
  ;[0.5 1 0.5] Game End Send Close
  (goto _label_2))

(event `CloseClean`
  ;[1 0.5 0.75] Close & Clean
  (bind _connectedport (`self.ConnectedPort`)
    (:`then`
      ;;[1 0 0 0.1 12] @REF - SerialCOM
      (`SerialCom.Flush` _connectedport)
      (bind _success (`self.SendMessageToPort` (`KismetStringLibrary.Concat_StrStr` "c" (`BlueprintMapLibrary.Map_Find` (`self.ACCESS_KEYS`) "Terminator")) _connectedport))
      (if _success
        ;;[1 0 0 0.1 12] @REF - SerialCOM
        (`SerialCom.Close` _connectedport)
        (set `self.ConnectedPort` null)
        (else
          (`KismetSystemLibrary.PrintText` "CONNECTED PORT FAILED WRITE" (`self.PrintingDebug`) true (struct :`R` 1.0 :`A` 1.0) 9999.0))))
    (:`else`)))

(event `StopReadSerial`
  (bind _readtimerhandle (`self.ReadTimerHandle`))
  ;[0.5 0.5 1] ReadSerial
  (if (`KismetSystemLibrary.K2_IsValidTimerHandle` _readtimerhandle)
    (`KismetSystemLibrary.K2_ClearAndInvalidateTimerHandle` _readtimerhandle)))

(event `ReadSerial`
  ;[0.5 0.5 1] ReadSerial
  (bind (_returnvalue _success) (`self.NewSerialRead` (`self.ConnectedPort`)))
  (if _success
    (bind _output_get (set `self.ArduinoOutput` _returnvalue))
    (if (> (`KismetStringLibrary.Len` _output_get) 0)
      (`self.Process` _output_get))))

(event `BeginReadSerial`
  ;[0.5 0.5 1] ReadSerial
  (bind _returnvalue (`KismetSystemLibrary.K2_SetTimerDelegate` (`|CreateDelegate` :!event `ReadSerial`) 0.001 true true))
  (set `self.ReadTimerHandle` _returnvalue))

(event `Process`
  (params (inString :type String))
  ;[0 1 1] @TODO Process Data
  (switch `string` (`KismetStringLibrary.ToUpper` (`KismetStringLibrary.Left` inString 1)) ; Switch on First Character - Type of Data
    (:`B`
      (`self.ButtonInputHandling` (`KismetStringLibrary.Conv_StringToInt` (`KismetStringLibrary.RightChop` inString 1))))
    (:`C`
      (switch `string` (`KismetStringLibrary.RightChop` inString 1)) ; Commands
    )))

(event `TestPortsForHandshake`
  (params (TestingID :type "Integer (by ref)") (PortsToCheck :type "Array of Integer (by ref)") (TestTimeDelay :type "Float (single-precision)" :default 2.5))
  ;[0.5 0.75 1] Recursively checks all supplied ports with a changeable testtime delay for initialisation
  (bind (_bopened _returnvalue) (`self.OpenPortForHandshake` PortsToCheck TestingID))
  (if _bopened
    (`KismetSystemLibrary.Delay` TestTimeDelay) ; InitTime
    (bind (_success _connectedport) (`self.TestPortForHandshake` (`self.PrintingDebug`) _returnvalue TestingID))
    (if _success
      (`self.ContinueExecutionWithBoundPort` _connectedport)
      (else
        (if (< TestingID (- (`KismetArrayLibrary.Array_Length` PortsToCheck) 1)) :!label _label_3
          (`self.TestPortsForHandshake` (+ TestingID 1) PortsToCheck)
          (else
            (`KismetSystemLibrary.PrintText` "NO PORT MATCHED HANDSHAKE KEY" (`self.PrintingDebug`) false (struct :`R` 1.0 :`A` 1.0) 100000.0)
            (`self.Failed`)))))
    (else
      (goto _label_3))))

(event `DEBUG_Override`
  (set `self.bOverride` true)
  (`/Game/Tools/BPFuncLib.DebugPrint` "ARDUINO CONNECTION OVERRIDE CALLED" (struct :`R` 1.0 :`B` 0.770756 :`A` 1.0) 20.0))

(fn `ButtonInputHandling`
  (params (ButtonData :type Integer))
  (`/Game/Tools/BPFuncLib.DebugPrint` (`|FormatText` "BUTTON STATE:  \n{bY} \n{bB} \n{bG} \n{bR}" (> (`KismetMathLibrary.And_IntInt` ButtonData 1) 0) (> (`KismetMathLibrary.And_IntInt` ButtonData 2) 0) (> (`KismetMathLibrary.And_IntInt` ButtonData 4) 0) (> (`KismetMathLibrary.And_IntInt` ButtonData 8) 0)) (struct :`G` 0.937471 :`B` 1.0 :`A` 1.0) 5.0 "ButtonStates"))

(fn `GetOpenablePorts`
  (params (MaxOpenablePorts :type Integer :default 16) (BaudRate :type Integer :default 9600))
  (returns (FoundPorts :type Boolean) (OpenablePorts :type "Array of Integer"))
  (locals (Local_OpenablePorts :type "Array of Integer"))
  (bind _local_openableports (`local.Local_OpenablePorts`))
  (for _index (range (+ MaxOpenablePorts 1))
    ;[1 0 0 0.1 12] @REF - SerialCOM
    (bind (_bopened _returnvalue) (`SerialCom.OpenComPort` _index BaudRate))
    (if _bopened
      (`KismetArrayLibrary.Array_Add` (`local.Local_OpenablePorts`) _index)
      ;[1 0 0 0.1 12] @REF - SerialCOM
      (`SerialCom.Close` _returnvalue)))
  (return (> (`KismetArrayLibrary.Array_Length` _local_openableports) 0) _local_openableports))

(fn `NewSerialRead`
  (params (Port :type "SerialCom Object Reference"))
  (returns (ReturnValue :type String) (Success :type Boolean))
  (`/Engine/EditorBlueprintResources/StandardMacros.IsValid` Port
    (:`Is Valid`
      (bind (_bsuccess _returnvalue) (`SerialCom.Readln` Port))
      (return (`KismetStringLibrary.Trim` _returnvalue) true))
    (:`Is Not Valid`
      (`/Game/Tools/BPFuncLib.DebugPrint` "SerialRead - Port Invalid" (struct :`R` 1.0 :`A` 1.0) 9999.0 "SerialPortInvalid")
      (return "" true))))

(fn `OpenPortForHandshake`
  (params (PortsToCheck :type "Array of Integer (by ref)") (TestingID :type "Integer (by ref)") (BaudRate :type Integer :default 9600))
  (returns (bOpened :type Boolean) (ReturnValue :type "SerialCom Object Reference"))
  (bind (_bopened _returnvalue) (`SerialCom.OpenComPortWithFlowControl` (`|GetArrayItem` PortsToCheck TestingID) BaudRate))
  (return _bopened _returnvalue))

(fn `ReadFromSerial`
  (params (ConnectedPort :type "SerialCom Object Reference") (ReturnsBlank :type Boolean))
  (returns (OutText :type String) (Success :type Boolean))
  (`/Engine/EditorBlueprintResources/StandardMacros.IsValid` ConnectedPort
    (:`Is Valid`
      ;[1 0 0 0.5 12] @REF - Serialcom
      (bind (_bsuccess _returnvalue) (`SerialCom.Readln` ConnectedPort))
      (if _bsuccess
        (if ReturnsBlank
          (bind _returnvalue_2 (`KismetStringLibrary.Trim` _returnvalue))
          (return _returnvalue_2 true)
          (else
            (return _returnvalue_2 (not (`KismetStringLibrary.EqualEqual_StrStr` _returnvalue_2)))))
        (else
          (`/Game/Tools/BPFuncLib.DebugPrint` "READ LINE FAIL" (struct :`R` 1.0 :`A` 1.0) 0.1 "ReadLineFail")
          (return "" false))))
    (:`Is Not Valid`
      (`/Game/Tools/BPFuncLib.DebugPrint` "PORT NOT VALID ON READ" (struct :`R` 1.0 :`A` 1.0) 9999.0 "InvalidPortOnRead")
      (return "" false))))

(fn `ReturnHandshake`
  (params (inPort :type "SerialCom Object Reference"))
  (returns (Success :type Boolean))
  (bind (_value _returnvalue) (`BlueprintMapLibrary.Map_Find` (`self.ACCESS_KEYS`) "HandshakeReturn"))
  (`/Engine/EditorBlueprintResources/StandardMacros.IsValid` inPort
    (:`Is Valid`
      (if _returnvalue
        (bind _success (`self.SendMessageToPort` _value inPort false))
        (return _success)
        (else
          (`/Game/Tools/BPFuncLib.DebugPrint` "Return Key Not Found" (struct :`R` 1.0 :`A` 1.0) 9999.0 "Return Key Not Found"))))
    (:`Is Not Valid`
      (return false))))

(fn `Send Message to Arduino`
  (params (CommandType :type String) (Parameters :type String))
  (returns (Success :type Boolean))
  (bind _connectedport (`self.ConnectedPort`)
    (:`then`
      (bind _success (`self.SendMessageToPort` (`KismetStringLibrary.Concat_StrStr` CommandType Parameters) _connectedport))
      (return _success))
    (:`else`
      (return false))))

(fn `SendMessageToPort`
  (params (String :type "Object Object Reference") (Port :type "SerialCom Object Reference") (isLine :type Boolean :default true))
  (returns (Success :type Boolean))
  (`/Engine/EditorBlueprintResources/StandardMacros.IsValid` Port
    (:`Is Valid`
      (if isLine
        ;[1 0 0 0.1 12] @REF - SerialCOM
        (bind _returnvalue (`SerialCom.Println` Port String))
        (if _returnvalue
          (return true)
          (else
            _))
        (else
          (bind _returnvalue_2 (`SerialCom.Print` Port String))
          (if _returnvalue_2
            (return true)
            (else
              _)))))
    (:`Is Not Valid`
      _))
  (return false))

(fn `TestPortForHandshake`
  (params (isPrintingDebug :type Boolean) (TestPort :type "SerialCom Object Reference") (TestingID :type Integer))
  (returns (Success :type Boolean) (ConnectedPort :type "SerialCom Object Reference"))
  (bind _returnvalue (`SerialCom.GetPort` TestPort))
  (`/Engine/EditorBlueprintResources/StandardMacros.IsValid` TestPort
    (:`Is Valid`
      (bind (_bsuccess _returnvalue_2) (`SerialCom.Readln` TestPort))
      (if _bsuccess
        (bind _returnvalue_3 (`KismetStringLibrary.Trim` _returnvalue_2))
        (if (`KismetStringLibrary.EqualEqual_StrStr` _returnvalue_3 (`BlueprintMapLibrary.Map_Find` (`self.ACCESS_KEYS`) "HandshakeOut"))
          (`KismetSystemLibrary.PrintText` (`|FormatText` "PORT_{id} CONNECTED SUCCESSFULLY" (`SerialCom.GetPort` TestPort)) (`local.isPrintingDebug`) false (struct :`G` 1.0 :`A` 1.0))
          (return true TestPort)
          (else
            (`KismetSystemLibrary.PrintText` (`|FormatText` "PORT_{ID} -> {TEXT}" _returnvalue _returnvalue_3) (`local.isPrintingDebug`) false (struct :`G` 0.66 :`B` 1.0 :`A` 1.0) 2.0 (`KismetStringLibrary.Conv_StringToName` (`KismetStringLibrary.Concat_StrStr` (`KismetStringLibrary.Conv_IntToString` _returnvalue) "PORTTEXT")))
            (return false null)))
        (else
          (`KismetSystemLibrary.PrintText` (`|FormatText` "PORT_{id} FAILED TO READ" (`SerialCom.GetPort` TestPort)) (`local.isPrintingDebug`) false (struct :`R` 1.0 :`A` 1.0) 100000.0))))
    (:`Is Not Valid`
      (`KismetSystemLibrary.PrintText` (`|FormatText` "PORT_{id} FAILED TO OPEN" (`SerialCom.GetPort` TestPort)) (`local.isPrintingDebug`) false (struct :`R` 1.0 :`A` 1.0) 100000.0)))
  (return false null))

(fn `UserConstructionScript`)