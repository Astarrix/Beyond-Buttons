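; PC_Main is the player controller that turns joystick input into astronaut thruster and yaw control.
; Init caches the astronaut pawn, its thruster component, HUD and Arduino interface from GM_MAIN, adds the joystick mapping context, then initialises the astronaut.
; Enhanced Input axes are inverted or remapped to set thruster direction, thrust with Niagara scale, and yaw rate.
; Debug keys trigger an Arduino override and toggle the astronaut camera.
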(event Custom|BindInput
  ;[1 1 0.5] Initialisation
  (Utilities|FlowControl|DelayUntilNextTick)
  (Input|AddMappingContext (PlayerController|LocalPlayerSubsystems|GetEnhancedInputLocalPlayerSubsystem) "/Game/Input/IMC_Joystick.IMC_Joystick" 0 (Utilities|Struct|MakeModifyContextOptions false true false)))

(event Custom|CreateReferences
  ;[1 1 0.5] Initialisation
  (bind _asbp_astronaut (Utilities|Casting|CastToBP_Astronaut (Pawn|GetControlledPawn))
    (:then
      (bind _output_get (Variables|References|SetAs%20BP%20Astronaut _asbp_astronaut))
      (bind _bpc_thrusters (Variables|/Game/Game/Player/BP_Astronaut.BP_Astronaut_C|GetBPC_Thrusters _output_get)
        (:then
          (Variables|Default|SetBPC%20Thrusters _bpc_thrusters)
          (bind _asgm_main (Utilities|Casting|CastToGM_MAIN (Game|GetGameMode))
            (:then
              (Variables|Default|SetHUD (Variables|/Game/Game/Core/GM_MAIN.GM_MAIN_C|GetHUD _asgm_main))
              (bind _arduinointerface (Variables|/Game/Game/Core/GM_MAIN.GM_MAIN_C|GetArduinoInterface _asgm_main)
                (:then
                  (Variables|References|SetArduinoInterface _arduinointerface))
                (:else
                  (CallFunction|DebugPrint "FAILED TO GATHER REFERENCES _ARDUINO" "(R=1.000000,G=0.000000,B=0.000000,A=1.000000)" 99999.0 "None"))))
            (:CastFailed
              (CallFunction|DebugPrint "FAILED TO GATHER REFERENCES _GAMEMODE" "(R=1.000000,G=0.000000,B=0.000000,A=1.000000)" 99999.0 "None"))))
        (:else
          (CallFunction|DebugPrint "FAILED TO GATHER REFERENCES _THRUSTER" "(R=1.000000,G=0.000000,B=0.000000,A=1.000000)" 99999.0 "None"))))
    (:CastFailed
      (CallFunction|DebugPrint "FAILED TO GATHER REFERENCES _ASTRONAUT" "(R=1.000000,G=0.000000,B=0.000000,A=1.000000)" 99999.0 "None"))))

(event Custom|Init
  ;[1 1 0.5] Initialisation
  (CallFunction|CreateReferences)
  (CallFunction|BindInput)
  (Default|Init (Variables|References|GetAs%20BP%20Astronaut)))

(event Input|EnhancedActionEvents|EnhancedInputActionIA_Rotate
  (params (ActionValue :type Float%20%28double-precision%29) (ElapsedSeconds :type Float%20%28double-precision%29) (TriggeredSeconds :type Float%20%28double-precision%29) (InputAction :type Input%20Action%20Object%20Reference :default "/Game/Input/JoystickInputs/IA_Rotate.IA_Rotate"))
  (bind __1___1 (Utilities|MaptoNegativeInclusive ActionValue))
  (bind _returnvalue (/ __1___1 5.0))
  ;[1 1 1] Rotate
  (CallFunction|DebugPrint (Utilities|Text|FormatText "Rotation Speed: {Val}" _returnvalue) "(R=0.000000,G=1.000000,B=0.314895,A=1.000000)" 0.1 "RotateInput")
  (Class|PlayerController|AddYawInput _returnvalue))

(event Input|EnhancedActionEvents|EnhancedInputActionIA_Direction
  (params (ActionValue :type Vector%202D%20Structure) (ElapsedSeconds :type Float%20%28double-precision%29) (TriggeredSeconds :type Float%20%28double-precision%29) (InputAction :type Input%20Action%20Object%20Reference :default "/Game/Input/JoystickInputs/IA_Direction.IA_Direction"))
  (bind (_x _y) (Math|Vector2D|BreakVector2D ActionValue))
  (bind _return (Utilities|OneMinus _y))
  (bind _return_2 (Utilities|OneMinus _x))
  (bind _out (Utilities|ChopFloat _return 2))
  (bind _out_2 (Utilities|ChopFloat _return_2 2))
  (bind __1___1 (Utilities|MaptoNegativeInclusive _out))
  (bind __1___1_2 (Utilities|MaptoNegativeInclusive _out_2))
  ;[0.5 0.5 1] Joystick Interaction
  (bind _bpc_thrusters (Variables|Default|GetBPC%20Thrusters)
    (:then
      (Variables|/Game/Game/Player/BPC_Thrusters.BPC_Thrusters_C|SetVelocityDirectionNormalizedWS _bpc_thrusters (Math|Vector|MakeVector __1___1_2 __1___1 0.0))
      (CallFunction|DebugPrint (Utilities|Text|FormatText "X: {x} 
Y: {y}" __1___1_2 __1___1) "(R=0.000000,G=1.000000,B=0.140181,A=1.000000)" 1.0 "Direction"))
    (:else)))

(event Input|EnhancedActionEvents|EnhancedInputActionIA_Thrust
  (params (ActionValue :type Float%20%28double-precision%29) (ElapsedSeconds :type Float%20%28double-precision%29) (TriggeredSeconds :type Float%20%28double-precision%29) (InputAction :type Input%20Action%20Object%20Reference :default "/Game/Input/JoystickInputs/IA_Thrust.IA_Thrust"))
  (bind _return (Utilities|OneMinus ActionValue))
  (bind _out (Utilities|ChopFloat _return 2))
  ;[0.5 0.5 1] Joystick Interaction
  (bind _bpc_thrusters (Variables|Default|GetBPC%20Thrusters)
    (:then
      (Development|PrintText (Utilities|Text|FormatText "Thrust: {fThrust}" _out) true false "(R=1.000000,G=0.000000,B=0.000000,A=1.000000)" 1e+01 "ThrustMapped")
      (if (!= (Variables|/Game/Game/Player/BPC_Thrusters.BPC_Thrusters_C|GetThrustPercentage _bpc_thrusters) _out)
        (bind _output_get (Variables|/Game/Game/Player/BPC_Thrusters.BPC_Thrusters_C|SetThrustPercentage _bpc_thrusters _out))
        (Niagara|SetNiagaraVariable(Float) (Variables|/Game/Game/Player/BPC_Thrusters.BPC_Thrusters_C|GetNS%20Thrusters _bpc_thrusters) "ThrustScale" _output_get)))
    (:else)))

(event Input|KeyboardEvents|DebugKeyK
  (params (Key :type Key%20Structure :default "None") (ActionValue :type Input%20Action%20Value%20Structure))
  ;[1 0.009595 0.3769] @DEBUG - Override
  (:Pressed
    (Default|DEBUGOverride (Variables|References|GetArduinoInterface))))

(event Input|KeyboardEvents|DebugKeyC
  (params (Key :type Key%20Structure :default "None") (ActionValue :type Input%20Action%20Value%20Structure))
  ;[1 0.009595 0.3769] @DEBUG - Override
  (:Pressed
    (bind _isa (Utilities|FlowControl|FlipFlop)
      (:A
        _)
      (:B
        _))
    (Default|SwitchCamera (Variables|References|GetAs%20BP%20Astronaut) _isa)))

(fn ConstructionScript)

(fn ReadInput
  (params (Key :type Key%20Structure%20%28by%20ref%29) (Value :type Input%20Action%20Value%20Structure))
  (bind _returnvalue (Class|KismetInputLibrary|KeyGetDisplayName Key true))
  (Development|PrintText (Utilities|Text|FormatText "KEY: {Name} 
Value: {Value}" _returnvalue (Utilities|String|ToString(Integer) Value)) true false "(R=0.000000,G=0.660000,B=1.000000,A=1.000000)" 2.0 (Utilities|String|StringToName (Utilities|String|ToString(Text) _returnvalue))))