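; Main game mode that sets up each level by name: the main menu on Level 0, and player input plus an Arduino connection on Level 1.
; On Level 1 it shows a loading widget and spawns the Arduino interface actor, whose search, retry and connected events drive that widget.
; On connection it removes the widget and sets cursor and input mode from the level name's last digit; EndPlay closes the interface cleanly.
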(event `self.ReceiveBeginPlay`
  (`self.CreateRefs`)
  (bind _returnvalue (`GameplayStatics.GetCurrentLevelName` true))
  (switch `string` _returnvalue
    (:`LEVEL_0`
      (bind _returnvalue_2 (`|CreateWidget` "/Game/UI/Widgets/UI_MainMenu.UI_MainMenu_C"))
      (`UserWidget.AddToViewport` _returnvalue_2 0))
    (:`LEVEL_1`
      (`/Game/Game/PC_Main.BindInput` (`self.As PC Main`))
      (`|ExecutionSequence`
        (:`then_0`
          (bind _returnvalue_3 (`|CreateWidget` "/Game/UI/Widgets/UI_ArduinoLoading.UI_ArduinoLoading_C"))
          (set `self.UI_LoadScreen` _returnvalue_3)
          (`UserWidget.AddToViewport` _returnvalue_3 2))
        (:`then_1`
          (`self.SpawnArduinoInterface`))))))

(event `CreateRefs`
  (set `self.As PC Main` (cast `/Game/Game/PC_Main` (`GameplayStatics.GetPlayerController` 0) :!pure true))
  (set `self.As PLAYERMAIN` (cast `/Game/Player/_PLAYERMAIN` (`GameplayStatics.GetPlayerPawn` 0) :!pure true)))

(event `SpawnArduinoInterface`
  (bind _returnvalue (`|SpawnActorFromClass` "/Game/ARDUINO/BP_ArduinoInterface.BP_ArduinoInterface_C" (`KismetMathLibrary.MakeTransform` (0.0 0.0 0.0)) "Undefined" "MultiplyWithRoot" null null))
  (bind _output_get (set `self.ArduinoInterface` _returnvalue))
  (add `/Game/ARDUINO/BP_ArduinoInterface.ED_BeginSearch` _output_get (`|CreateDelegate` :!event `ArduinoBeginSearch`))
  (add `/Game/ARDUINO/BP_ArduinoInterface.ED_Retrying` _output_get (`|CreateDelegate` :!event `ArduinoRetryConnection`))
  (add `/Game/ARDUINO/BP_ArduinoInterface.ED_Connected` _output_get (`|CreateDelegate` :!event `ArduinoConnected`))
  (`/Game/ARDUINO/BP_ArduinoInterface.Init` _output_get))

(event `self.ReceiveEndPlay`
  (params (EndPlayReason :type "EEndPlayReason Enum" :default "Destroyed"))
  (bind _arduinointerface (`self.ArduinoInterface`)
    (:`then`
      (`/Game/ARDUINO/BP_ArduinoInterface.CloseClean` _arduinointerface))
    (:`else`)))

(event `ArduinoConnected`
  (bind _returnvalue (`GameplayStatics.GetPlayerController` 0))
  (bind _ui_loadscreen (`self.UI_LoadScreen`)
    (:`then`
      (`Widget.RemoveFromParent` _ui_loadscreen)
      (bind _returnvalue_2 (`GameplayStatics.GetCurrentLevelName` true))
      (bind _returnvalue_3 (select `int` (`KismetStringLibrary.Conv_StringToInt` (`KismetStringLibrary.Right` _returnvalue_2 1)) :`0` false :`1` true))
      (set `PlayerController.bShowMouseCursor` _returnvalue_3 _returnvalue)
      (if _returnvalue_3
        (`WidgetBlueprintLibrary.SetInputMode_GameAndUIEx` _returnvalue null)
        (else
          (`WidgetBlueprintLibrary.SetInputMode_GameOnly` _returnvalue))))
    (:`else`)))

(event `ArduinoBeginSearch`
  (bind _ui_loadscreen (`self.UI_LoadScreen`)
    (:`then`
      (`/Game/UI/Widgets/UI_ArduinoLoading.DisplayPanel` _ui_loadscreen true))
    (:`else`)))

(event `ArduinoRetryConnection`
  (bind _ui_loadscreen (`self.UI_LoadScreen`)
    (:`then`
      (`/Game/UI/Widgets/UI_ArduinoLoading.DisplayPanel` _ui_loadscreen false))
    (:`else`)))

(fn `UserConstructionScript`)