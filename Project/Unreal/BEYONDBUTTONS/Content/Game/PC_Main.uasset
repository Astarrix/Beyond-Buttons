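; Main player controller that drives the player pawn's movement, jump and look, and handles interaction and joystick input testing.
; BeginPlay caches the pawn and GM_MAIN's Arduino interface, used by a debug key to send a test serial message.
; Interact actions send InteractionMessage to actors hit by camera or cursor traces.
; BindInput adds the joystick mapping context; joystick actions and raw USB axes print values for debugging, some through BitwiseSign.
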(event Custom|BindInput
  ;[1 1 0.5] Initialisation
  (Input|AddMappingContext (PlayerController|LocalPlayerSubsystems|GetEnhancedInputLocalPlayerSubsystem) "/Game/Input/IMC_Joystick.IMC_Joystick" 0 (Utilities|Struct|MakeModifyContextOptions true false false)))

(event Custom|CreateReferences
  ;[1 1 0.5] Initialisation
  (bind _as_playermain (Utilities|Casting|CastTo_PLAYERMAIN (Pawn|GetControlledPawn)))
  (Variables|Default|SetAs%20PLAYER _as_playermain)
  (bind _asgm_main (Utilities|Casting|CastToGM_MAIN (Game|GetGameMode)))
  (Variables|Default|SetArduinoInterface (Variables|/Game/Game/GM_MAIN.GM_MAIN_C|GetArduinoInterface _asgm_main)))

(event Input|EnhancedActionEvents|EnhancedInputActionIA_2DMove
  (params (ActionValue :type Vector%202D%20Structure) (ElapsedSeconds :type Float%20%28double-precision%29) (TriggeredSeconds :type Float%20%28double-precision%29) (InputAction :type Input%20Action%20Object%20Reference :default "/Game/Input/InputActions/IA_2DMove.IA_2DMove"))
  (bind (_x _y) (Math|Vector2D|BreakVector2D ActionValue))
  (bind _as_player (Variables|Default|GetAs%20PLAYER))
  ;[1 0.5 0.5] Movement
  (Pawn|Input|AddMovementInput _as_player (Transformation|GetActorForwardVector _as_player) _y false)
  (Pawn|Input|AddMovementInput _as_player (Transformation|GetActorRightVector _as_player) _x false))

(event Input|EnhancedActionEvents|EnhancedInputActionIA_Jump
  (params (ActionValue :type Boolean) (ElapsedSeconds :type Float%20%28double-precision%29) (TriggeredSeconds :type Float%20%28double-precision%29) (InputAction :type Input%20Action%20Object%20Reference :default "/Game/Input/InputActions/IA_Jump.IA_Jump"))
  (bind _as_player (Variables|Default|GetAs%20PLAYER))
  ;[1 0.5 0.5] Movement
  (:Triggered
    (Character|Jump _as_player))
  (:Canceled
    (Character|StopJumping _as_player :!label _label))
  (:Completed
    (goto _label)))

(event Input|EnhancedActionEvents|EnhancedInputActionIA_Interact
  (params (ActionValue :type Boolean) (ElapsedSeconds :type Float%20%28double-precision%29) (TriggeredSeconds :type Float%20%28double-precision%29) (InputAction :type Input%20Action%20Object%20Reference :default "/Game/Input/InputActions/IA_Interact.IA_Interact"))
  (bind _as_player (Variables|Default|GetAs%20PLAYER))
  (bind _camera (Variables|/Game/Player/_PLAYERMAIN._PLAYERMAIN_C|GetCamera _as_player))
  ;[1 0.5 1] Interaction
  (:Started
    (bind (_success _location _hitactor _hitcomponent) (CallFunction|LineTrace (Transformation|GetWorldLocation _camera) (Math|Vector|GetForwardVector _camera) 1e+03 "None"))
    (if _success
      (Class|BPI|Interaction(Message) _hitactor (Variables|Default|GetAs%20PLAYER) _hitcomponent))))

(event Input|EnhancedActionEvents|EnhancedInputActionIA_Look
  (params (ActionValue :type Vector%202D%20Structure) (ElapsedSeconds :type Float%20%28double-precision%29) (TriggeredSeconds :type Float%20%28double-precision%29) (InputAction :type Input%20Action%20Object%20Reference :default "/Game/Input/InputActions/IA_Look.IA_Look"))
  (bind (_x _y) (Math|Vector2D|BreakVector2D ActionValue))
  ;[1 0.5 0.5] Movement
  (Class|PlayerController|AddPitchInput (* _y -1.0))
  (Class|PlayerController|AddYawInput _x))

(event Input|EnhancedActionEvents|EnhancedInputActionIA_MouseInteraction
  (params (ActionValue :type Boolean) (ElapsedSeconds :type Float%20%28double-precision%29) (TriggeredSeconds :type Float%20%28double-precision%29) (InputAction :type Input%20Action%20Object%20Reference :default "/Game/Input/InputActions/IA_MouseInteraction.IA_MouseInteraction"))
  (bind (_hitresult _returnvalue) (Game|Player|GetHitResultUnderCursorbyChannel "TraceTypeQuery1" true))
  (bind (_bblockinghit _binitialoverlap _time _distance _location _impactpoint _normal _impactnormal _physmat _hitactor _hitcomponent) (Collision|BreakHitResult _hitresult))
  (:Started
    (if _returnvalue
      (Class|BPI|Interaction(Message) _hitactor (Variables|Default|GetAs%20PLAYER) _hitcomponent)
      (Development|PrintString (Utilities|GetDisplayName _hitactor)))))

(event Input|EnhancedActionEvents|EnhancedInputActionIA_Direction
  (params (ActionValue :type Vector%202D%20Structure) (ElapsedSeconds :type Float%20%28double-precision%29) (TriggeredSeconds :type Float%20%28double-precision%29) (InputAction :type Input%20Action%20Object%20Reference :default "/Game/Input/JoystickInputs/IA_Direction.IA_Direction"))
  (bind (_x _y) (Math|Vector2D|BreakVector2D ActionValue))
  ;[0.5 0.5 1] Joystick Interaction
  (Development|PrintText (Utilities|Text|FormatText "X: {x} 
Y: {y}" (Utilities|BitwiseSign _x) (Utilities|BitwiseSign _y)) true true "(R=0.000000,G=0.660000,B=1.000000,A=1.000000)" 2.0 "move"))

(event Input|EnhancedActionEvents|EnhancedInputActionIA_Thrust
  (params (ActionValue :type Float%20%28double-precision%29) (ElapsedSeconds :type Float%20%28double-precision%29) (TriggeredSeconds :type Float%20%28double-precision%29) (InputAction :type Input%20Action%20Object%20Reference :default "/Game/Input/JoystickInputs/IA_Thrust.IA_Thrust"))
  ;[0.5 0.5 1] Joystick Interaction
  (Development|PrintText (Utilities|Text|FormatText "Thrust: {fThrust}" (Utilities|BitwiseSign ActionValue)) true false "(R=1.000000,G=0.000000,B=0.000000,A=1.000000)" 1e+01 "ThrustMapped"))

(event EventBeginPlay
  ;[1 1 0.5] Initialisation
  (CallFunction|CreateReferences))

(event Input|KeyboardEvents|DebugKey6
  (params (Key :type Key%20Structure :default "None") (ActionValue :type Input%20Action%20Value%20Structure))
  ;[1 1 0.5] Initialisation
  (:Pressed
    (bind _arduinointerface (Variables|Default|GetArduinoInterface)
      (:then
        (Default|SendMessagetoPort _arduinointerface "p63TESTTEXT" (Variables|/Game/ARDUINO/BP_ArduinoInterface.BP_ArduinoInterface_C|GetConnectedPort _arduinointerface)))
      (:else))))

(event Input|KeyboardEvents|DebugKeyM
  (params (Key :type Key%20Structure :default "None") (ActionValue :type Input%20Action%20Value%20Structure))
  (:Pressed
    (CallFunction|ReadInput Key)))

(event Input|KeyboardEvents|DebugKeyGenericUSBControllerAxis7
  (params (Key :type Key%20Structure :default "None") (ActionValue :type Input%20Action%20Value%20Structure))
  (:Pressed
    (CallFunction|ReadInput Key ActionValue)))

(event Input|KeyboardEvents|DebugKeyGenericUSBControllerAxis5
  (params (Key :type Key%20Structure :default "None") (ActionValue :type Input%20Action%20Value%20Structure))
  (:Pressed
    (CallFunction|ReadInput Key ActionValue)))

(event Input|KeyboardEvents|DebugKeyGenericUSBControllerAxis6
  (params (Key :type Key%20Structure :default "None") (ActionValue :type Input%20Action%20Value%20Structure))
  (:Pressed
    (CallFunction|ReadInput Key ActionValue)))

(event Input|KeyboardEvents|DebugKeyGenericUSBControllerAxis1
  (params (Key :type Key%20Structure :default "None") (ActionValue :type Input%20Action%20Value%20Structure))
  (:Pressed
    (CallFunction|ReadInput Key ActionValue)))

(event Input|KeyboardEvents|DebugKeyGenericUSBControllerAxis2
  (params (Key :type Key%20Structure :default "None") (ActionValue :type Input%20Action%20Value%20Structure))
  (:Pressed
    (CallFunction|ReadInput Key ActionValue)))

(event Input|KeyboardEvents|DebugKeyGenericUSBControllerAxis3
  (params (Key :type Key%20Structure :default "None") (ActionValue :type Input%20Action%20Value%20Structure))
  (:Pressed
    (CallFunction|ReadInput Key ActionValue)))

(event Input|KeyboardEvents|DebugKeyGenericUSBControllerAxis4
  (params (Key :type Key%20Structure :default "None") (ActionValue :type Input%20Action%20Value%20Structure))
  (:Pressed
    (CallFunction|ReadInput Key ActionValue)))

(event Input|KeyboardEvents|DebugKeyGenericUSBControllerAxis8
  (params (Key :type Key%20Structure :default "None") (ActionValue :type Input%20Action%20Value%20Structure))
  (:Pressed
    (CallFunction|ReadInput Key ActionValue)))

(fn ConstructionScript)

(fn ReadInput
  (params (Key :type Key%20Structure%20%28by%20ref%29) (Value :type Input%20Action%20Value%20Structure))
  (bind _returnvalue (Class|KismetInputLibrary|KeyGetDisplayName Key true))
  (Development|PrintText (Utilities|Text|FormatText "KEY: {Name} 
Value: {Value}" _returnvalue (Utilities|String|ToString(Integer) Value)) true false "(R=0.000000,G=0.660000,B=1.000000,A=1.000000)" 2.0 (Utilities|String|StringToName (Utilities|String|ToString(Text) _returnvalue))))