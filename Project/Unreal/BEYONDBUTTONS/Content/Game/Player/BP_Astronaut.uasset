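; BP_Astronaut is the player astronaut, managing an oxygen supply that drains over time and mirroring it to Arduino hardware.
; Init sets up the thrusters component, fetches the Arduino interface from GM_MAIN and starts a looping one-second timer.
; Each tick lowers oxygen as a percentage of tank duration and sends the truncated value to the Arduino.
; At empty, it stops the timer, signals the Arduino and calls the OxygenDepleted dispatcher.
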(event `Init`
  (`self.Create References`)
  (`self.BeginOxygenDegredation`))

(event `Create References`
  (`/Game/Game/Player/BPC_Thrusters.Init` (`self.BPC_Thrusters`) self)
  (bind _output_get (set `self.As GM MAIN` (cast `/Game/Game/Core/GM_MAIN` (`GameplayStatics.GetGameMode`) :!pure true)))
  (bind _arduinointerface (`/Game/Game/Core/GM_MAIN.ArduinoInterface` _output_get)
    (:`then`
      (set `self.Arduino Interface` _arduinointerface))
    (:`else`
      (`/Game/Tools/BPFuncLib.DebugPrint` "ASTRONAUT FAILED TO GET REFERENCE TO ARDUINO"))))

(event `BeginOxygenDegredation`
  (bind _returnvalue (`KismetSystemLibrary.K2_SetTimerDelegate` (delegate `DegradeOxygen`) 1.0 true true))
  (set `self.Oxygen_TimerHandle` _returnvalue))

(event `DegradeOxygen`
  (if (not (<= (`self.OxygenRemaining`) 0.0))
    (bind _output_get (set `self.OxygenRemaining` (- (`self.OxygenRemaining`) (/ 100.0 (`self.OxygenMaxTankTime_Seconds`)))))
    (`/Game/Game/Core/BP_ArduinoInterface.Send Message to Arduino` (`self.Arduino Interface`) "t" (`KismetStringLibrary.Conv_IntToString` (`KismetMathLibrary.FTrunc` _output_get)))
    (else
      (`self.StopOxygenTimer`)
      (`/Game/Game/Core/BP_ArduinoInterface.Send Message to Arduino` (`self.Arduino Interface`) "b" "")
      (`self.ED_OxygenDepleted`))))

(event `StopOxygenTimer`
  (bind _oxygen_timerhandle (`self.Oxygen_TimerHandle`))
  (if (`KismetSystemLibrary.K2_IsValidTimerHandle` _oxygen_timerhandle)
    (`KismetSystemLibrary.K2_ClearAndInvalidateTimerHandle` _oxygen_timerhandle)))

(fn `UserConstructionScript`)