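; Actor component that gives BP_Astronaut limited-fuel thruster movement.
; It caches the astronaut owner on BeginPlay, and EngageThrusters starts a fast looping timer for the thrust tick.
; Each MovementOnThruster call burns fuel and adds movement input along a stored direction, scaled by thrust percentage.
; When fuel runs out it calls DisengageThrusters, which clears the timer; nothing here sets the direction or refills fuel.
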(event `self.ReceiveBeginPlay`
  (`self.CreateReferences`))

(event `CreateReferences`
  (bind _asbp_astronaut (cast `/Game/Game/Player/BP_Astronaut` (`self.GetOwner`)))
  (set `self.As BP Astronaut` _asbp_astronaut))

(event `EngageThrusters`
  (bind _returnvalue (`KismetSystemLibrary.K2_SetTimerDelegate` (`|CreateDelegate` :!event `MovementOnThruster`) 0.01 true true))
  (set `self.Thruster_TimerHandle` _returnvalue))

(event `MovementOnThruster`
  (if (> (`self.Thrust_Remaining`) 0.0)
    (set `self.Thrust_Remaining` (- (`self.Thrust_Remaining`) (`self.Thrust_BurnPerTick`)))
    (`Pawn.AddMovementInput` (`self.As BP Astronaut`) (`self.VelocityDirectionNormalized`) (`self.ThrustPercentage`) false)
    (else
      (`self.DisengageThrusters`))))

(event `DisengageThrusters`
  (bind _thruster_timerhandle (`self.Thruster_TimerHandle`))
  (if (`KismetSystemLibrary.K2_IsValidTimerHandle` _thruster_timerhandle)
    (`KismetSystemLibrary.K2_ClearAndInvalidateTimerHandle` _thruster_timerhandle)))